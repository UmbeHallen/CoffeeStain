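; BP_Enemy is an enemy character that wakes when the player approaches and can be lifted off the ground by balloons.
; Player overlap with its sphere activates the behavior tree once, via a message to its controller.
; EnableFlight, called by BP_Balloon, sets Flying, disables gravity, enables physics and stops the AI logic.
; DisableFlight restores gravity only; paired DoOnce gates re-arm each other, ignoring duplicate calls from multiple balloons.
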(event `self.Sphere.OnComponentBeginOverlap`
  (params (OverlappedComponent :type "PrimitiveComponent Object Reference") (OtherActor :type "Actor Object Reference") (OtherComp :type "PrimitiveComponent Object Reference") (OtherBodyIndex :type Integer) (bFromSweep :type Boolean) (SweepResult :type "HitResult Structure (by ref)"))
  ;[1 1 1] Run behavior tree.
  (if (== OtherActor (`GameplayStatics.GetPlayerCharacter` 0))
    (`/Engine/EditorBlueprintResources/StandardMacros.DoOnce` false ; Only executes once.
      (:`Completed`
        (message `/Game/WackyGame/Utility/Interfaces/Enemy/BPI_Enemy.ActivateBehaviorTree` (`self.GetController`)) ; Activates this character's brain.
      ))))

(event `/Game/WackyGame/Utility/Interfaces/Enemy/BPI_Enemy.EnableFlight`
  (bind _returnvalue (`AIBlueprintHelperLibrary.GetAIController` null))
  ;[0 0.1061 1] Fly with balloons
  ;;[1 1 1] Talks to behavior tree to prevent continued movement.
  (`/Engine/EditorBlueprintResources/StandardMacros.DoOnce` false :!label _label ; Only executes once (there might be multiple balloons enforcing the same command).
    (:`Completed`
      (set `self.Flying?` true) ; Set flying to true (checked by AI behavior).
      ;;[1 1 1] Enable flight.
      (`PrimitiveComponent.SetEnableGravity` (`self.CapsuleComponent`) false)
      (`PrimitiveComponent.SetEnableGravity` (`self.Mesh`) false)
      (`PrimitiveComponent.SetEnableGravity` (`self.Sphere`) false) ; Enables character to be able to leave the ground.
      (`PrimitiveComponent.SetSimulatePhysics` (`self.CapsuleComponent`) true)
      (`PrimitiveComponent.SetSimulatePhysics` (`self.Mesh`) true)
      (`PrimitiveComponent.SetSimulatePhysics` (`self.Sphere`) true) ; Enables character to be able to leave the ground.
      (`self.ResetGrounded`) ; Enables character to fall if needed.
      ;;[1 1 1] Stop behavior tree.
      (`/Engine/EditorBlueprintResources/StandardMacros.IsValid` _returnvalue ; Checks if brain is still running.
        (:`Is Valid`
          (`BrainComponent.StopLogic` (`AIController.BrainComponent` _returnvalue) "") ; Stop running behavior tree logic.
        )))))

(event `ResetFlight`
  ;[0 0.1061 1] Fly with balloons
  (goto _label :!via `Reset`))

(event `/Game/WackyGame/Utility/Interfaces/Enemy/BPI_Enemy.DisableFlight`
  ;[1 0.2132 0] Fall to the ground
  (`/Engine/EditorBlueprintResources/StandardMacros.DoOnce` false :!label _label_2 ; Only executes once (there might be multiple balloons enforcing the same command).
    (:`Completed`
      ;;[1 1 1] Disable flight.
      (`PrimitiveComponent.SetEnableGravity` (`self.CapsuleComponent`) true)
      (`PrimitiveComponent.SetEnableGravity` (`self.Mesh`) true)
      (`PrimitiveComponent.SetEnableGravity` (`self.Sphere`) true) ; Enables character to be able to leave the ground.
      (`self.ResetFlight`) ; Enables character to fly if needed.
    )))

(event `ResetGrounded`
  ;[1 0.2132 0] Fall to the ground
  (goto _label_2 :!via `Reset`))

(fn `GetFlying`
  (returns (`Flying?` :type Boolean))
  (return (`self.Flying?`)))

(fn `UserConstructionScript`)