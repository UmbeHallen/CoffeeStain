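; BP_BalloonProjectile is a randomly colored projectile that turns into an attached balloon on impact.
; A looping timer runs a small, zero-length sphere trace at the mesh, ignoring the player.
; On a hit, it spawns a BP_Balloon, passes it the hit component, bone and color, registers it with the player character and destroys itself.
; The first missed trace starts a five-second delay that destroys stray projectiles.
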(event `self.ReceiveBeginPlay`
  ;[1 0.04831 0] Hit event
  ;;[1 1 1] Continuously traces for obstacles.
  (bind _returnvalue (`KismetSystemLibrary.K2_SetTimerDelegate` (delegate `TraceForImpact`) 0.03 true)) ; Starts a looping timer.
  (set `self.TraceForImpactEvent` _returnvalue) ; Saving the variable for later manipulation.
  ;;[1 1 1] Set mesh material.
  (set `self.BalloonColor` (select `int` (`KismetMathLibrary.RandomIntegerInRange` 0 3) :`0` "/Game/WackyGame/Materials/M_Red.M_Red" :`1` "/Game/WackyGame/Materials/M_Blue.M_Blue" :`2` "/Game/WackyGame/Materials/M_Green.M_Green" :`3` "/Game/WackyGame/Materials/M_Yellow.M_Yellow" :!type "MaterialInterface Object Reference")) ; Returns a random color from the selection of materials.
  (`PrimitiveComponent.SetMaterial` (`self.ProjectileMesh`) 0 (`self.BalloonColor`)) ; Sets the mesh's material to the randomized color.
)

(event `TraceForImpact`
  (bind _returnvalue (`SceneComponent.K2_GetComponentLocation` (`self.ProjectileMesh`)))
  ;[1 0.04831 0] Hit event
  ;;[1 1 1] Continuously traces for obstacles.
  (bind (_outhit _returnvalue_2) (`KismetSystemLibrary.SphereTraceSingle` _returnvalue _returnvalue 10.0 "TraceTypeQuery1" false (`|MakeArray` (`GameplayStatics.GetPlayerCharacter` 0) :!type "Actor Object Reference") "None" true (struct :`R` 1.0 :`A` 1.0) (struct :`G` 1.0 :`A` 1.0) 0.5)) ; Trace for obstacles.
  (if _returnvalue_2
    ;;[1 1 1] Stops the trace for objects.
    (`KismetSystemLibrary.K2_ClearAndInvalidateTimerHandle` (`self.TraceForImpactEvent`)) ; Stops- the looping timer.
    (bind (_bblockinghit _binitialoverlap _time _distance _location _impactpoint _normal _impactnormal _physmat _hitactor _hitcomponent _hitbonename) (`GameplayStatics.BreakHitResult` _outhit))
    ;;[1 1 1] Spawns a balloon at the hit location.
    (bind _returnvalue_3 (`|SpawnActorFromClass` "/Game/WackyGame/Blueprints/Balloon/BP_Balloon.BP_Balloon_C" (`KismetMathLibrary.MakeTransform` _location) "AdjustIfPossibleButAlwaysSpawn" "OverrideRootScale" null null)) ; Spawns a BP_Balloon at the hit location.
    ;;[1 1 1] Sends hit information to spawned balloon and sets its color.
    (`/Game/WackyGame/Blueprints/Balloon/BP_Balloon.AttachBalloon` _returnvalue_3 _location _hitcomponent _hitbonename) ; Sends hit info to the spawned BP_Balloon.
    (message `/Game/WackyGame/Utility/Interfaces/Balloon/BPI_Balloon.SetColor` _returnvalue_3 (`self.BalloonColor`)) ; Sends material color to the spawned BP_Balloon.
    ;;[1 1 1] Adds spawned balloon to player's array.
    (message `/Game/WackyGame/Utility/Interfaces/Characters/BPI_WackyCharacter.AddBalloon` (`GameplayStatics.GetPlayerCharacter` 0) _returnvalue_3) ; Sends the spawned actor to BP_WackyCharacter to be stored in an array.
    ;;[1 1 1] Destroys the projectile.
    (`self.K2_DestroyActor`) ; Destroys this projectile.
    (else
      ;;[1 1 1] Destroy projectiles that don't hit anything.
      (`KismetSystemLibrary.Delay` 5.0) ; If the projectile doesn't hit anything for a while it is destroyed.
      (`self.K2_DestroyActor`))))

(fn `UserConstructionScript`)